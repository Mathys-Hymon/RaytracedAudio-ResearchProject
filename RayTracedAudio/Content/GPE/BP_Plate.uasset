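; BP_Plate is a trigger plate that slides up to five referenced wall actors toward itself and back.
; On BeginPlay it caches each valid wall's start position and an end position DistanceWalls along the direction to the plate.
; Any Box begin-overlap alternates, via FlipFlop, between playing and reversing the LerpPosition timeline, which lerps the walls between those positions by teleporting without sweep.
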(event `self.ReceiveBeginPlay`
  (bind _leftwall (`self.LeftWall`))
  (bind _upwall (`self.UpWall`))
  (bind _rightwall (`self.RightWall`))
  (bind _frontwall (`self.FrontWall`))
  (bind _backwall (`self.BackWall`))
  (`/Engine/EditorBlueprintResources/StandardMacros.IsValid` _leftwall
    (:`Is Valid`
      (set `self.initialLeftWallPos` (`self.K2_GetActorLocation` _leftwall))
      (set `self.endLeftWallPos` (`self.WallPosToEndPos` _leftwall)))
    (:`Is Not Valid`
      _))
  (`/Engine/EditorBlueprintResources/StandardMacros.IsValid` _upwall
    (:`Is Valid`
      (set `self.initialUpWallPos` (`self.K2_GetActorLocation` _upwall))
      (set `self.endUpWallPos` (`self.WallPosToEndPos` _upwall)))
    (:`Is Not Valid`
      _))
  (`/Engine/EditorBlueprintResources/StandardMacros.IsValid` _rightwall
    (:`Is Valid`
      (set `self.initialRightWallPos` (`self.K2_GetActorLocation` _rightwall))
      (set `self.EndRightWallPos` (`self.WallPosToEndPos` _rightwall)))
    (:`Is Not Valid`
      _))
  (`/Engine/EditorBlueprintResources/StandardMacros.IsValid` _frontwall
    (:`Is Valid`
      (set `self.initialFrontWallPos` (`self.K2_GetActorLocation` _frontwall))
      (set `self.endFrontWallPos` (`self.WallPosToEndPos` _frontwall)))
    (:`Is Not Valid`
      _))
  (`/Engine/EditorBlueprintResources/StandardMacros.IsValid` _backwall
    (:`Is Valid`
      (set `self.initialBackWallPos` (`self.K2_GetActorLocation` _backwall))
      (set `self.endBackWallPos` (`self.WallPosToEndPos` _backwall)))))

(event `self.Box.OnComponentBeginOverlap`
  (params (OverlappedComponent :type "PrimitiveComponent Object Reference") (OtherActor :type "Actor Object Reference") (OtherComp :type "PrimitiveComponent Object Reference") (OtherBodyIndex :type Integer) (bFromSweep :type Boolean) (SweepResult :type "HitResult Structure (by ref)"))
  (bind _backwall (`self.BackWall`))
  (bind _rightwall (`self.RightWall`))
  (bind _frontwall (`self.FrontWall`))
  (bind _leftwall (`self.LeftWall`))
  (bind _upwall (`self.UpWall`))
  (`/Engine/EditorBlueprintResources/StandardMacros.FlipFlop`
    (:`A`
      (bind (_direction _alpha) (`Timeline|LerpPosition` :!label _label)
        (:`Update`
          (`/Engine/EditorBlueprintResources/StandardMacros.IsValid` _leftwall
            (:`Is Valid`
              (`self.K2_SetActorLocation` _leftwall (`KismetMathLibrary.VLerp` (`self.initialLeftWallPos`) (`self.endLeftWallPos`) _alpha) false true))
            (:`Is Not Valid`
              _))
          (`/Engine/EditorBlueprintResources/StandardMacros.IsValid` _upwall
            (:`Is Valid`
              (`self.K2_SetActorLocation` _upwall (`KismetMathLibrary.VLerp` (`self.initialUpWallPos`) (`self.endUpWallPos`) _alpha) false true))
            (:`Is Not Valid`
              _))
          (`/Engine/EditorBlueprintResources/StandardMacros.IsValid` _rightwall
            (:`Is Valid`
              (`self.K2_SetActorLocation` _rightwall (`KismetMathLibrary.VLerp` (`self.initialRightWallPos`) (`self.EndRightWallPos`) _alpha) false true))
            (:`Is Not Valid`
              _))
          (`/Engine/EditorBlueprintResources/StandardMacros.IsValid` _frontwall
            (:`Is Valid`
              (`self.K2_SetActorLocation` _frontwall (`KismetMathLibrary.VLerp` (`self.initialFrontWallPos`) (`self.endFrontWallPos`) _alpha) false true))
            (:`Is Not Valid`
              _))
          (`/Engine/EditorBlueprintResources/StandardMacros.IsValid` _backwall
            (:`Is Valid`
              (`self.K2_SetActorLocation` _backwall (`KismetMathLibrary.VLerp` (`self.initialBackWallPos`) (`self.endBackWallPos`) _alpha) false true))))))
    (:`B`
      (goto _label :!via `Reverse`))))

(fn `UserConstructionScript`)

(fn `WallPosToEndPos`
  (params (wallActor :type "Actor Object Reference"))
  (returns (endPos :type "Vector Structure"))
  (bind _returnvalue (`self.K2_GetActorLocation` wallActor))
  (return (+ _returnvalue (* (`KismetMathLibrary.Normal` (- (`self.K2_GetActorLocation`) _returnvalue)) (`self.distanceWalls`)))))
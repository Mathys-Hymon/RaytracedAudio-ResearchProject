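; Actor component that visualises its owner's sound as decals, showing where bouncing sound paths reach BPI_Sound actors.
; An arrow component sweeps a sphere of directions, one randomly offset ring per tick, firing reflecting line traces with a shared distance budget.
; Direct hits mark the impact, bounced hits mark the preceding bounce point, scaled by remaining distance.
; A half-second timer batches marks into one Niagara system via arrays, with material chosen by SoundType.
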(event `self.ReceiveBeginPlay`
  (bind _returnvalue (`|AddComponentByClass` :`self` (`self.GetOwner`) :`Class` "/Script/Engine.ArrowComponent"))
  (set `self.Arrow` _returnvalue)
  (`KismetSystemLibrary.K2_SetTimerDelegate` (delegate `UpdateNiagara`) 0.5 true true)
  (`self.UpdateTrace`))

(event `UpdateTrace`
  (bind _traceamount (`self.traceAmount`))
  (bind (_returnvalue_roll _returnvalue_pitch _returnvalue_yaw) (`KismetMathLibrary.BreakRotator` (`SceneComponent.K2_GetComponentRotation` (`self.Arrow`))))
  (bind _index (`self.ForLoopDelay` 0 _traceamount)
    (:`loopBody`
      (bind _returnvalue (* (`KismetMathLibrary.Conv_IntToDouble` _index) (/ 180.0 (`KismetMathLibrary.Conv_IntToDouble` _traceamount))))
      (`SceneComponent.K2_SetWorldRotation` (`self.Arrow`) (`KismetMathLibrary.MakeRotator` _returnvalue_roll _returnvalue _returnvalue_yaw) false false)
      (bind _returnvalue_2 (`KismetMathLibrary.RandomFloatInRange` -88.0 88.0))
      (bind _returnvalue_3 (- (`self.traceAmount`) (`KismetMathLibrary.Lerp` (`KismetMathLibrary.Conv_IntToDouble` (`self.traceAmount`)) 0.0 (/ (`KismetMathLibrary.Abs` (- _returnvalue 90.0)) 90.0))))
      (for _index_2 (range (+ _returnvalue_3 1))
        (`SceneComponent.K2_SetWorldRotation` (`self.Arrow`) (`KismetMathLibrary.MakeRotator` _returnvalue_roll _returnvalue_pitch (+ _returnvalue_2 (`KismetMathLibrary.Conv_IntToDouble` (* _index_2 (/ 360 _returnvalue_3))))) false false)
        (`self.CalculateAudioBounce` (`Actor.K2_GetActorLocation` (`self.GetOwner`)) (`SceneComponent.GetForwardVector` (`self.Arrow`)) (`self.soundDistanceTrace`) (`self.maxBounces`) 20.0)))
    (:`completed`
      (`KismetSystemLibrary.DelayUntilNextTick`)
      (`self.UpdateTrace`))))

(event `UpdateNiagara`
  ; V3
  (if (!= (`KismetArrayLibrary.Array_Length` (`self.decalsToSpawn`)) 0)
    (bind _returnvalue (`NiagaraFunctionLibrary.SpawnSystemAtLocation` "/Game/Material/FX/NS_Decals.NS_Decals" (`Actor.K2_GetActorLocation` (`self.GetOwner`)) (struct) (1.0 1.0 1.0) true true "AutoRelease"))
    (`NiagaraComponent.SetVariableMaterial` _returnvalue "MaterialTexture" (select `/Game/Data/Enum_SoundType` (`self.soundType`) :`NewEnumerator0` "/Game/Material/FX/MI_FXEnemy.MI_FXEnemy" :`NewEnumerator1` "/Game/Material/FX/MI_FXShoot.MI_FXShoot" :`NewEnumerator2` "/Game/Material/FX/MI_FXMusic.MI_FXMusic" :`NewEnumerator3` "/Game/Material/FX/MI_FXFootsteps.MI_FXFootsteps" :`NewEnumerator5` "/Game/Material/FX/MI_FXArrow.MI_FXArrow" :!type "MaterialInterface Object Reference"))
    (`NiagaraComponent.SetNiagaraVariableInt` _returnvalue "HitCount" (`KismetArrayLibrary.Array_Length` (`self.decalsToSpawn`)))
    (`NiagaraDataInterfaceArrayFunctionLibrary.SetNiagaraArrayVector` _returnvalue "HitLocations" (`self.decalsPos`))
    (`NiagaraDataInterfaceArrayFunctionLibrary.SetNiagaraArrayVector` null "HitFacings" (`self.decalsFacing`))
    (`NiagaraDataInterfaceArrayFunctionLibrary.SetNiagaraArrayFloat` _returnvalue "HitScales" (`self.decalsScale`))
    (`NiagaraComponent.SetVariableFloat` _returnvalue "DecalDuration" (`self.decalLifeTime`))
    (`NiagaraDataInterfaceArrayFunctionLibrary.SetNiagaraArrayQuat` _returnvalue "HitRotations" (`self.decalsRotation`))
    (`KismetArrayLibrary.Array_Clear` (`self.decalsToSpawn`))
    (`KismetArrayLibrary.Array_Clear` (`self.decalsPos`))
    (`KismetArrayLibrary.Array_Clear` (`self.decalsScale`))
    (`KismetArrayLibrary.Array_Clear` (`self.decalsRotation`))
    (`KismetArrayLibrary.Array_Clear` (`self.decalsFacing`))))

(fn `CalculateAudioBounce`
  (params (initialPos :type "Vector Structure") (initialDir :type "Vector Structure") (soundDistance :type "Float (double-precision)" :default 2000.0) (maxBounces :type Integer) (decalSize :type "Float (double-precision)"))
  (locals (currentPos :type "Vector Structure") (currentDir :type "Vector Structure") (distanceLeft :type "Float (double-precision)" :default 3000.0) (endPos :type "Vector Structure") (previousSize :type "Float (double-precision)") (previousRot :type "Rotator Structure" :default (struct)) (previousDecalFacing :type "Vector Structure"))
  (bind _returnvalue (* (/ (`local.distanceLeft`) (`local.soundDistance`)) (`local.decalSize`)))
  (set `local.currentPos` initialPos)
  (set `local.currentDir` initialDir)
  (set `local.distanceLeft` soundDistance)
  (for _index (range (+ maxBounces 1))
    (set `local.endPos` (+ (`local.currentPos`) (* (`local.currentDir`) (`local.distanceLeft`))))
    (bind (_outhit _returnvalue_2) (`KismetSystemLibrary.LineTraceSingle` :`Start` (`local.currentPos`) :`End` (`local.endPos`) :`TraceChannel` "TraceTypeQuery1" :`DrawDebugType` (select `bool` (`self.showDebug`) :`true` "ForDuration" :!type "EDrawDebugTrace Enum") :`DrawTime` (`self.updateSpeed`)))
    (if _returnvalue_2
      (bind (_bblockinghit _binitialoverlap _time _distance _location _impactpoint _normal _impactnormal _physmat _hitactor) (`GameplayStatics.BreakHitResult` _outhit))
      (`/Engine/EditorBlueprintResources/StandardMacros.IsValid` _hitactor
        (:`Is Valid`
          (if (`KismetSystemLibrary.DoesImplementInterface` _hitactor "/Game/BP/BPI_Sound.BPI_Sound_C")
            (if (== _index 0)
              (`|ExecutionSequence`
                (:`then_0`
                  _)
                (:`then_1`
                  (`KismetArrayLibrary.Array_Add` (`self.decalsToSpawn`) (make `/Game/Data/S_DecalsData` (`KismetMathLibrary.Conv_DoubleToVector` _returnvalue) (stale _output_get) (stale _output_get_2) (`self.updateSpeed`)) :!label _label)
                  (set `local.previousSize` _returnvalue)
                  (`KismetArrayLibrary.Array_Add` (`self.decalsPos`) (stale _output_get))
                  (`KismetArrayLibrary.Array_Add` (`self.decalsScale`) (* _returnvalue (`self.decalScale`)))
                  (`KismetArrayLibrary.Array_Add` (`self.decalsRotation`) (`KismetMathLibrary.Conv_RotatorToQuaternion` (stale _output_get_2)))
                  (`KismetArrayLibrary.Array_Add` (`self.decalsFacing`) (`local.previousDecalFacing`))))
              (set `local.distanceLeft` (- (`local.distanceLeft`) _distance) :!label _label_2)
              (bind _output_get (set `local.currentPos` (+ _impactpoint (* _impactnormal 2.0))))
              (set `local.currentDir` (`KismetMathLibrary.GetReflectionVector` (`local.currentDir`) _impactnormal))
              (bind _output_get_2 (set `local.previousRot` (`KismetMathLibrary.MakeRotFromXZ` (* _impactnormal -1.0) (- (`Actor.K2_GetActorLocation` (`self.GetOwner`)) _impactpoint))))
              (set `local.previousDecalFacing` _impactnormal)
              (else
                (`|ExecutionSequence`
                  (:`then_0`
                    (goto _label))
                  (:`then_1`
                    (set `local.distanceLeft` 0.0)))))
            (else
              (goto _label_2))))
        (:`Is Not Valid`
          (goto _label_2)))
      (else
        (break)))))